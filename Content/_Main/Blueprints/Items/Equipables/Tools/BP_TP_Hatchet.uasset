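; Equippable hatchet that chops harvestable large items and damages other actors.
; Use plays first- and third-person montages; its notify gets the owner's arrow transform for a server sphere overlap.
; Large items lose health and yield data-table resources, randomly scaled by tool type, tier and damage, or get replaced by a spawned actor at zero health, with multicast hit effects.
; Other targets take damage, reduced by armor piece count on survival characters.
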(event Custom|GetRotationClient
  (bind (_location _rotation) (Class|BPISurvivalCharacter|GetArrowLocation(Message) (Components|GetOwner)))
  (CallFunction|ServerOverlap _location _rotation))

(event Custom|ServerOverlap
  (params (SpherePos :type Vector) (Rotation :type Rotator))
  (bind (_outactors _returnvalue) (Collision|SphereOverlapActors SpherePos 6e+01 (Utilities|Array|MakeArray "ObjectTypeQuery8" "ObjectTypeQuery3") 0 (Utilities|Array|MakeArray (Variables|Default|GetChar%20Ref))))
  (if _returnvalue
    (for _array_element _outactors
      (bind _damage (CallFunction|CalculateDamage _array_element (Math|Conversions|ToFloat(Integer) (Utilities|Struct|BreakS_ItemInfo (Variables|Default|GetitemInfo)))))
      (if (Utilities|DoesObjectImplementInterface _array_element "/Game/_Main/Blueprints/Interfaces/BPI_Largeltem.BPI_Largeltem_C")
        (CallFunction|HarvestFoliage _damage _array_element)
        (CallFunction|HitFXMulticast SpherePos Rotation)
        (else
          (Game|Damage|ApplyDamage _array_element _damage (Pawn|GetController (Variables|Default|GetChar%20Ref)) self "/Script/Engine.DamageType"))))))

(event Custom|HitFXMulticast
  (params (Location :type Vector) (Rotation :type Rotator))
  (bind _outhit (Collision|LineTraceByChannel Location (+ Location (* (Math|Vector|GetForwardVector Rotation) (Variables|Default|GetTraceDistance))) "TraceTypeQuery1" false 0 "None"))
  (Effects|SpawnEmitteratLocation "/Game/Realistic_Starter_VFX_Pack_Vol2/Particles/Hit/P_PickaxeHit.P_PickaxeHit" (.ImpactPoint (Collision|BreakHitResult _outhit)))
  (Audio|PlaySoundatLocation (Variables|Default|GethitSound) Location "0, 0, 0" 1.0 1.0 0.0 "/Game/_Main/Sounds/Harvesting/HarvestingAtt.HarvestingAtt" 0 0 0))

(event EventBeginPlay
  (|CallParentFunction) ; This node is disabled and will not be called.\nDrag off pins to build functionality.
)

(event Collision|EventActorBeginOverlap
  (params (OtherActor :type Actor%20Object%20Reference))
  (|CallParentFunction OtherActor) ; This node is disabled and will not be called.\nDrag off pins to build functionality.
)

(event EventTick
  (params (DeltaSeconds :type Float%20%28single-precision%29))
  (|CallParentFunction DeltaSeconds) ; This node is disabled and will not be called.\nDrag off pins to build functionality.
)

(event EventUselteminterface
  (params (CharRef :type BP%20First%20Person%20Character%20Object%20Reference))
  (if (not (Variables|Default|GetIsSwinging?))
    (Variables|Default|SetIsSwinging? true)
    (bind _output_get (Variables|Default|SetChar%20Ref CharRef))
    (Class|BPISurvivalCharacter|FirstPersonMontage(Message) _output_get "/Game/Man/Animations/Hatchet_Chop_Montage.Hatchet_Chop_Montage")
    (Class|BPISurvivalCharacter|ThirdPersonMontage(Message) _output_get "/Game/Man/Animations/Hatchet_Chop_Montage.Hatchet_Chop_Montage")))

(event EventEndAnimation
  (Variables|Default|SetIsSwinging? false))

(event EventNotifyInterface
  (CallFunction|GetRotationClient))

(fn ConstructionScript
  (|CallParentFunction))

(fn HarvestFoliage
  (params (damage :type Float%20%28double-precision%29) (ref :type Actor%20Object%20Reference))
  (bind _ref (Class|BPILargeltem|GetLargeltemRef(Message) ref))
  (Utilities|IsValid _ref
    (:Is%20Valid
      (bind _output_get (Variables|/Game/_Main/Blueprints/HarvestingSystem/BP_HarvestingMaster.BP_HarvestingMaster_C|Sethealth _ref (- (Variables|/Game/_Main/Blueprints/HarvestingSystem/BP_HarvestingMaster.BP_HarvestingMaster_C|Gethealth _ref) damage)))
      (bind _returnvalue (Utilities|GetDataTableRow "/Game/_Main/Blueprints/DataTables/DT_LargeltemResources.DT_LargeltemResources" (Utilities|String|StringToName (Utilities|GetClassDisplayName (Utilities|GetClass _ref))))
        (:then
          (if (<= _output_get 0.0)
            (Game|SpawnActorfromClass (.Class (Utilities|Struct|BreakS_Largeltem _returnvalue)) (Transformation|GetActorTransform _ref) "Undefined" 0 (Transformation|GetActorForwardVector (Variables|Default|GetChar%20Ref)) 0)
            (Actor|DestroyActor _ref)
            (else
              (for _array_element (.Givenitema (Utilities|Struct|BreakS_Largeltem _returnvalue))
                (if (not (<= (Math|Float|Truncate (|((((BaseVar*RateVar)*ToolTypeVar)*ToolTierVar)*DamageVar) (Math|Conversions|ToFloat(Integer) (.Quantity (Utilities|Struct|BreakS_ResourceStructures _array_element))) 1.0 (Math|Float|SelectFloat (Math|Random|RandomFloatinRange 0.2 0.4) (Math|Random|RandomFloatinRange 0.01 0.1) (Utilities|Enum|Equal(Enum) (.PrefferedToolType (Utilities|Struct|BreakS_ResourceStructures _array_element)) (Variables|Default|GetToolType))) (Utilities|Select :Index (Variables|Default|GetToolTier) :NewEnumerator0 (Math|Random|RandomFloatinRange 0.8 1.2) :NewEnumerator1 (Math|Random|RandomFloatinRange 1.2 1.6)) damage)) 0))
                  (bind _survivalcharref (Class|BPISurvivalCharacter|GetSurvivalCharRef(Message) (Variables|Default|GetChar%20Ref)))
                  (Default|HarvestItemonServer _survivalcharref (Utilities|Struct|MakeS_ResourceStructures (.ResourcelD (Utilities|Struct|BreakS_ResourceStructures _array_element)) (Math|Float|Truncate (|((((BaseVar*RateVar)*ToolTypeVar)*ToolTierVar)*DamageVar) (Math|Conversions|ToFloat(Integer) (.Quantity (Utilities|Struct|BreakS_ResourceStructures _array_element))) 1.0 (Math|Float|SelectFloat (Math|Random|RandomFloatinRange 0.2 0.4) (Math|Random|RandomFloatinRange 0.01 0.1) (Utilities|Enum|Equal(Enum) (.PrefferedToolType (Utilities|Struct|BreakS_ResourceStructures _array_element)) (Variables|Default|GetToolType))) (Utilities|Select :Index (Variables|Default|GetToolTier) :NewEnumerator0 (Math|Random|RandomFloatinRange 0.8 1.2) :NewEnumerator1 (Math|Random|RandomFloatinRange 1.2 1.6)) damage)) "NewEnumerator0")))))))))))

(fn CalculateDamage
  (params (HitActor :type Actor%20Object%20Reference) (ItemBaseDamage :type Float%20%28double-precision%29))
  (LocalVariables|SetlocalDamage (* ItemBaseDamage (Variables|Default|GetDamageMultiplier)))
  (if (Utilities|DoesObjectImplementInterface HitActor "/Game/_Main/Blueprints/Interfaces/BPI_SurvivalCharacter.BPI_SurvivalCharacter_C")
    (bind _totalarmorsiot (Class|BPISurvivalCharacter|GetTotalArmorPieces(Message) HitActor))
    (switch int _totalarmorsiot
      (:0
        (return (* (LocalVariables|GetlocalDamage) 4.0)))
      (:1
        (return (* (LocalVariables|GetlocalDamage) 3.5)))
      (:2
        (return (* (LocalVariables|GetlocalDamage) 3.0)))
      (:3
        (return (* (LocalVariables|GetlocalDamage) 2.5)))
      (:4
        (return (* (LocalVariables|GetlocalDamage) 2.0))))
    (else
      (return (* (LocalVariables|GetlocalDamage) 4.0)))))