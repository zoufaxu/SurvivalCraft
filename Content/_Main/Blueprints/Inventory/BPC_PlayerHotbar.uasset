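; Player hotbar component that specializes a parent item container for the character's hotbar slots.
; Slot drops are accepted from the player inventory or hotbar via TransferItem, and CheckHotbar reports whether a slot is filled and its item type.
; Add and remove overrides call the parent, then update the slot through the owner's controller.
; Any removal also tells the survival character to dequip its current item, without checking which slot was equipped.
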(event EventBeginPlay
  (|CallParentFunction) ; This node is disabled and will not be called.\nDrag off pins to build functionality.
)

(event EventTick
  (params (DeltaSeconds :type Float%20%28single-precision%29))
  (|CallParentFunction DeltaSeconds) ; This node is disabled and will not be called.\nDrag off pins to build functionality.
)

(fn CheckHotbar
  (params (index :type Integer))
  (bind _items (Variables|Default|GetItems))
  (bind _output (Utilities|Array|Get(acopy) _items index))
  (return (!= (.itemid _output) 0) (.itemtype _output)))

(fn HandleSlotDrop
  (params (FromContainer :type BPC%20Items%20Container%20Object%20Reference) (Fromindex :type Integer) (Droppedindex :type Integer))
  (switch Utilities|FlowControl|Switch|SwitchonE_ContainerType (Variables|/Game/_Main/Blueprints/Inventory/BPC_ItemsContainer.BPC_ItemsContainer_C|GetContainerType FromContainer)
    (:NewEnumerator0
      _)
    (:NewEnumerator1
      _))
  (Default|TransferItem FromContainer self Droppedindex Fromindex))

(fn AddItemtoIndex
  (params (item :type S%20Item%20Info%20Structure) (LocalSpecificindex :type Integer) (Fromindex :type Integer))
  (bind _success_ (|CallParentFunction item LocalSpecificindex Fromindex))
  (bind _controllerref (Class|BPISurvivalCharacter|GetControllerfromChar(Message) (Components|GetOwner)))
  (Default|UpdateItemSlot _controllerref (Variables|Default|GetContainerType) LocalSpecificindex (CallFunction|GetItematIndex LocalSpecificindex))
  (return _success_))

(fn RemoveItematIndex
  (params (index :type Integer))
  (|CallParentFunction index)
  (bind _controllerref (Class|BPISurvivalCharacter|GetControllerfromChar(Message) (Components|GetOwner)))
  (Default|ResetItemSlot _controllerref (Variables|Default|GetContainerType) index)
  (bind _survivalcharref (Class|BPISurvivalCharacter|GetSurvivalCharRef(Message) (Components|GetOwner)))
  (Default|DequipCurrentitem _survivalcharref))