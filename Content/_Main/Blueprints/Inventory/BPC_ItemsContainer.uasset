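; Base inventory container component that holds an array of item slots, with ItemID 0 marking an empty slot.
; AddItem tops up matching stacks, then spills the remainder into empty slots; companion functions check, remove and transfer items between containers.
; UpdateUI forwards slot changes for Player Inventory and Hotbar types to the owner's controller through interface messages.
; AddItemOnServer and OnSlotDrop events wrap AddItem and HandleSlotDrop, which is empty here.
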(event Custom|AddItemOnServer
  (params (Item :type S%20Item%20Info%20Structure))
  (CallFunction|AddItem Item))

(event Custom|OnSlotDrop
  (params (FromContainer :type BPC%20Items%20Container%20Object%20Reference) (Fromindex :type Integer) (Droppedindex :type Integer))
  (CallFunction|HandleSlotDrop FromContainer Fromindex Droppedindex))

(event EventBeginPlay)

(event EventTick
  (params (DeltaSeconds :type Float%20%28single-precision%29)))

(fn FindEmptySlot
  (bind (_array_element _array_index) (Utilities|Array|ForEachLoopwithBreak (Variables|Default|GetItems) :!label _label)
    (:LoopBody
      (if (== (Utilities|Struct|BreakS_ItemInfo _array_element) 0)
        (LocalVariables|SetEmptySlotIndex _array_index)
        (LocalVariables|SetFonfEmptySlot? true)
        (goto _label Break)))
    (:Completed
      (return (LocalVariables|GetFonfEmptySlot?) (LocalVariables|GetEmptySlotIndex)))))

(fn AddItem
  (params (Item :type S%20Item%20Info%20Structure))
  (bind (_itemid _itemquantity) (Utilities|Struct|BreakS_ItemInfo Item))
  (bind _output_get (LocalVariables|SetlocalItemInfo Item))
  (if (Utilities|Struct|BreakS_ItemInfo _output_get)
    (bind _itemexistsininv_ (CallFunction|HasItemstoStack? Item))
    (if _itemexistsininv_
      (bind (_array_element _array_index) (Utilities|Array|ForEachLoopwithBreak (Variables|Default|GetItems))
        (:LoopBody
          (if (and (== (.ItemID (Utilities|Struct|BreakS_ItemInfo _array_element)) _itemid) (< (.ItemQuantity (Utilities|Struct|BreakS_ItemInfo _array_element)) (.StackSize (Utilities|Struct|BreakS_ItemInfo _array_element))))
            (LocalVariables|SetmaxStackSize (.StackSize (Utilities|Struct|BreakS_ItemInfo _array_element)))
            (LocalVariables|SetemptyIndex _array_index)
            (bind _output_get_2 (LocalVariables|SetCurrentSlotQuantity (.ItemQuantity (Utilities|Struct|BreakS_ItemInfo _array_element))))
            (LocalVariables|SetTempSlotQuantity _output_get_2)
            (LocalVariables|SetTotalltemQuantity _itemquantity)
            (bind _output_get_3 (LocalVariables|SetCurrentSlotQuantity (Math|Integer|SelectInt (LocalVariables|GetmaxStackSize) (+ (LocalVariables|GetCurrentSlotQuantity) (LocalVariables|GetTotalltemQuantity)) (>= (+ (LocalVariables|GetCurrentSlotQuantity) (LocalVariables|GetTotalltemQuantity)) (LocalVariables|GetmaxStackSize)))))
            (bind _structout (Utilities|Struct|SetmembersinS_ItemInfo (LocalVariables|GetlocalItemInfo) _output_get_3))
            (Utilities|Array|SetArrayElem (Variables|Default|GetItems) (LocalVariables|GetemptyIndex) _structout)
            (CallFunction|UpdateUI (LocalVariables|GetemptyIndex) _structout false)
            (Utilities|Struct|SetmembersinS_ItemInfo (LocalVariables|GetlocalItemInfo) (Math|Integer|SelectInt (Math|Integer|Clamp(Integer) (- (LocalVariables|GetTotalltemQuantity) (- (LocalVariables|GetmaxStackSize) (LocalVariables|GetTempSlotQuantity))) 0 (LocalVariables|GetTotalltemQuantity)) 0 (>= (+ (LocalVariables|GetCurrentSlotQuantity) (LocalVariables|GetTotalltemQuantity)) (LocalVariables|GetmaxStackSize))))))
        (:Completed
          (if (> (Utilities|Struct|BreakS_ItemInfo (LocalVariables|GetlocalItemInfo)) 0)
            (if (> (.ItemQuantity (Utilities|Struct|BreakS_ItemInfo (LocalVariables|GetlocalItemInfo))) (.StackSize (Utilities|Struct|BreakS_ItemInfo (LocalVariables|GetlocalItemInfo)))) :!label _label
              (LocalVariables|SetTotalltemQuantity (.ItemQuantity (Utilities|Struct|BreakS_ItemInfo (LocalVariables|GetlocalItemInfo))))
              (LocalVariables|SetmaxStackSize (.StackSize (Utilities|Struct|BreakS_ItemInfo (LocalVariables|GetlocalItemInfo))))
              (bind (_success_ _emptyindex) (CallFunction|FindEmptySlot :!label _label_2))
              (if _success_
                (LocalVariables|SetemptyIndex _emptyindex)
                (LocalVariables|SetCurrentSlotQuantity 0)
                (LocalVariables|SetTempSlotQuantity 0)
                (bind _output_get_4 (LocalVariables|SetCurrentSlotQuantity (Math|Integer|SelectInt (LocalVariables|GetmaxStackSize) (+ (LocalVariables|GetCurrentSlotQuantity) (LocalVariables|GetTotalltemQuantity)) (>= (+ (LocalVariables|GetCurrentSlotQuantity) (LocalVariables|GetTotalltemQuantity)) (LocalVariables|GetmaxStackSize)))))
                (bind _structout_2 (Utilities|Struct|SetmembersinS_ItemInfo (LocalVariables|GetlocalItemInfo) _output_get_4))
                (Utilities|Array|SetArrayElem (Variables|Default|GetItems) (LocalVariables|GetemptyIndex) _structout_2)
                (CallFunction|UpdateUI (LocalVariables|GetemptyIndex) _structout_2 false)
                (bind _output_get_5 (LocalVariables|SetTotalltemQuantity (Math|Integer|SelectInt (Math|Integer|Clamp(Integer) (- (LocalVariables|GetTotalltemQuantity) (- (LocalVariables|GetmaxStackSize) (LocalVariables|GetTempSlotQuantity))) 0 (LocalVariables|GetTotalltemQuantity)) 0 (>= (+ (LocalVariables|GetCurrentSlotQuantity) (LocalVariables|GetTotalltemQuantity)) (LocalVariables|GetmaxStackSize)))))
                (if (> _output_get_5 0)
                  (goto _label_2)
                  (else
                    (return true)))
                (else
                  (return true)))
              (else
                (bind (_success__2 _emptyindex_2) (CallFunction|FindEmptySlot :!label _label_3))
                (if _success__2
                  (Utilities|Array|SetArrayElem (Variables|Default|GetItems) _emptyindex_2 Item)
                  (CallFunction|UpdateUI _emptyindex_2 Item false)
                  (return true)
                  (else
                    (return false)))))
            (else
              (return true)))))
      (else
        (goto _label)))
    (else
      (goto _label_3))))

(fn UpdateUI
  (params (index :type Integer) (itemInfo :type S%20Item%20Info%20Structure) (resetSlot? :type Boolean))
  (if resetSlot?
    (switch Utilities|FlowControl|Switch|SwitchonE_ContainerType (Variables|Default|GetContainerType)
      (:NewEnumerator0
        _)
      (:NewEnumerator1
        _))
    (bind _controllerref (Class|BPISurvivalCharacter|GetControllerfromChar(Message) (Components|GetOwner)))
    (Default|ResetItemSlot _controllerref (Variables|Default|GetContainerType) index)
    (else
      (switch Utilities|FlowControl|Switch|SwitchonE_ContainerType (Variables|Default|GetContainerType)
        (:NewEnumerator0
          _)
        (:NewEnumerator1
          _))
      (bind _controllerref_2 (Class|BPISurvivalCharacter|GetControllerfromChar(Message) (Components|GetOwner)))
      (Default|UpdateItemSlot _controllerref_2 (Variables|Default|GetContainerType) index itemInfo))))

(fn HandleSlotDrop
  (params (FromContainer :type BPC%20Items%20Container%20Object%20Reference) (Fromindex :type Integer) (Droppedindex :type Integer)))

(fn TransferItem
  (params (ToComponent :type BPC%20Items%20Container%20Object%20Reference) (ToSpecificindex :type Integer) (ItemindexToTranfser :type Integer))
  (Utilities|IsValid ToComponent
    (:Is%20Valid
      (bind _success_ (CallFunction|AddItemtoIndex ToComponent (CallFunction|GetItematIndex ItemindexToTranfser) ToSpecificindex ItemindexToTranfser))
      (if _success_
        (CallFunction|RemoveItematIndex ItemindexToTranfser)))))

(fn GetItematIndex
  (params (index :type Integer))
  (if (Utilities|Array|IsValidIndex (Variables|Default|GetItems) index)
    (return (Utilities|Array|Get(acopy) (Variables|Default|GetItems) index))
    (else
      (return ""))))

(fn AddItemtoIndex
  (params (item :type S%20Item%20Info%20Structure) (LocalSpecificindex :type Integer) (Fromindex :type Integer))
  (if (CallFunction|IsSlotEmpty? LocalSpecificindex)
    (Utilities|Array|SetArrayElem (Variables|Default|GetItems) LocalSpecificindex item)
    (return true)
    (else
      (return false))))

(fn IsSlotEmpty?
  (params (slotIndex :type Integer))
  (return (== (.itemid (Utilities|Array|Get(acopy) (Variables|Default|GetItems) slotIndex)) 0)))

(fn RemoveItematIndex
  (params (index :type Integer))
  (Utilities|Array|SetArrayElem :TargetArray (Variables|Default|GetItems) :Index index))

(fn HasItemstoStack?
  (params (itemInfo :type S%20Item%20Info%20Structure))
  (bind _array_element (Utilities|Array|ForEachLoopwithBreak (Variables|Default|GetItems) :!label _label)
    (:LoopBody
      (if (and (== (.ItemID (Utilities|Struct|BreakS_ItemInfo _array_element)) (Utilities|Struct|BreakS_ItemInfo itemInfo)) (< (.ItemQuantity (Utilities|Struct|BreakS_ItemInfo _array_element)) (.StackSize (Utilities|Struct|BreakS_ItemInfo _array_element))))
        (LocalVariables|SetExistsInInventory true)
        (goto _label Break)))
    (:Completed
      (return (LocalVariables|GetExistsInInventory)))))

(fn ContainsItems
  (params (items :type Array%20of%20S%20Item%20Struct%20Structures))
  (bind _output_get (LocalVariables|SetHasItems? items))
  (bind _array_element (Utilities|Array|ForEachLoopwithBreak _output_get)
    (:LoopBody
      (bind _array_element_2 (Utilities|Array|ForEachLoopwithBreak (Variables|Default|GetItems))
        (:LoopBody
          (if (and (== (.ItemID (Utilities|Struct|BreakS_ItemStruct _array_element)) (.ItemID (Utilities|Struct|BreakS_ItemInfo _array_element_2))) (>= (.ItemQuantity (Utilities|Struct|BreakS_ItemStruct _array_element)) (.ItemQuantity (Utilities|Struct|BreakS_ItemInfo _array_element_2))))
            (bind (_array_element_3 _array_index) (Utilities|Array|ForEachLoopwithBreak (LocalVariables|GetHasItems?))
              (:LoopBody
                (if (== (Utilities|Struct|BreakS_ItemStruct _array_element_3) (.ItemID (Utilities|Struct|BreakS_ItemStruct _array_element)))
                  (Utilities|Array|RemoveIndex (LocalVariables|GetHasItems?) _array_index))))))
        (:Completed
          (return (Utilities|Array|IsEmpty (LocalVariables|GetHasItems?))))))))

(fn RemoveItems
  (params (itemsToRemove :type Array%20of%20S%20Item%20Struct%20Structures))
  (bind _array_element (Utilities|Array|ForEachLoopwithBreak itemsToRemove)
    (:LoopBody
      (LocalVariables|SetqutntityToRemove (.ItemQuantity (Utilities|Struct|BreakS_ItemStruct _array_element)))
      (bind _indexes (CallFunction|GetIndexesOfItems (.ItemID (Utilities|Struct|BreakS_ItemStruct _array_element))))
      (bind _array_element_2 (Utilities|Array|ForEachLoopwithBreak _indexes :!label _label)
        (:LoopBody
          (bind _output_get (LocalVariables|SetslotIndex _array_element_2))
          (if (<= (- (Utilities|Struct|BreakS_ItemInfo (Utilities|Array|Get(acopy) (Variables|Default|GetItems) _output_get)) (LocalVariables|GetqutntityToRemove)) 0)
            (LocalVariables|SetqutntityToRemove (- (LocalVariables|GetqutntityToRemove) (- (Utilities|Struct|BreakS_ItemInfo (Utilities|Array|Get(acopy) (Variables|Default|GetItems) _output_get)) (LocalVariables|GetqutntityToRemove))))
            (Utilities|Array|SetArrayElem :TargetArray (Variables|Default|GetItems) :Index (LocalVariables|GetslotIndex))
            (CallFunction|UpdateUI :index (LocalVariables|GetslotIndex) :resetSlot? true)
            (if (== (LocalVariables|GetqutntityToRemove) 0)
              (goto _label Break))
            (else
              (bind _structout (Utilities|Struct|SetmembersinS_ItemInfo (Utilities|Array|Get(acopy) (Variables|Default|GetItems) (LocalVariables|GetslotIndex)) (- (Utilities|Struct|BreakS_ItemInfo (Utilities|Array|Get(acopy) (Variables|Default|GetItems) (LocalVariables|GetslotIndex))) (LocalVariables|GetqutntityToRemove))))
              (Utilities|Array|SetArrayElem (Variables|Default|GetItems) (LocalVariables|GetslotIndex) _structout)
              (CallFunction|UpdateUI (LocalVariables|GetslotIndex) _structout false)
              (goto _label Break))))))))

(fn GetIndexesOfItems
  (params (ItemID :type Integer))
  (bind (_array_element _array_index) (Utilities|Array|ForEachLoopwithBreak (Variables|Default|GetItems))
    (:LoopBody
      (if (and (== (.ItemID (Utilities|Struct|BreakS_ItemInfo _array_element)) ItemID) (> (.ItemQuantity (Utilities|Struct|BreakS_ItemInfo _array_element)) 0))
        (Utilities|Array|Add (LocalVariables|GetindexesFound) _array_index)))
    (:Completed
      (return (LocalVariables|GetindexesFound)))))

(fn UpdateltemQuantity
  (params (index :type Integer) (NewQuantity :type Integer))
  (bind _structout (Utilities|Struct|SetmembersinS_ItemInfo (Utilities|Array|Get(acopy) (Variables|Default|GetItems) index) NewQuantity))
  (Utilities|Array|SetArrayElem (Variables|Default|GetItems) index _structout)
  (if (<= NewQuantity 0)
    (CallFunction|RemoveItematIndex index)
    (return true)
    (else
      (CallFunction|UpdateUI index _structout false)
      (return false))))

(fn RemoveQuantity
  (params (index :type Integer) (amountToRemove :type Integer))
  (bind _output_get (LocalVariables|SetcurrentQuantity (Utilities|Struct|BreakS_ItemInfo (Utilities|Array|Get(acopy) (Variables|Default|GetItems) index))))
  (bind _removeorupdate_ (CallFunction|UpdateltemQuantity index (- _output_get amountToRemove)))
  (return _removeorupdate_ (LocalVariables|GetcurrentQuantity)))