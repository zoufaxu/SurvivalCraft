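; Player preview actor that renders an equippable character mesh through a scene capture into a material handed to the controller.
; Equip events spawn items onto sockets and armor onto the mesh, using leader pose to sync armor animation.
; Item dequip destroys the held actor.
; Armor dequip branches share one destroy call targeting chest, pants and boots together, never the helmet.
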(event Custom|InializeWindow
  (params (CoontrollerRef :type Survival%20Game%20PC%20Object%20Reference))
  (bind _returnvalue (Rendering|CreateRenderTarget2D 500 800 "RTF_RGBA16f"))
  (Variables|/Script/Engine.SceneCaptureComponent2D|SetTextureTarget (Variables|Default|GetSceneCaptureComponent2D) _returnvalue)
  (bind _returnvalue_2 (Rendering|Material|CreateDynamicMaterialInstance "/Game/_Main/Blueprints/PlayerWindow/M_PlayerMaterial.M_PlayerMaterial" "None" "None" :!class /Script/Engine.KismetMaterialLibrary))
  (Rendering|Material|SetTextureParameterValue _returnvalue_2 "Param" _returnvalue)
  (Utilities|IsValid CoontrollerRef
    (:Is%20Valid
      (Default|SetRenderMaterial CoontrollerRef _returnvalue_2))))

(event Custom|EquipltemEvent
  (params (info :type S%20Equipable%20Info%20Structure))
  (bind (_socketname _animationstate _firstpersonequipclass) (Utilities|Struct|BreakS_EquipableInfo info))
  (Variables|Default|SetEquippedState _animationstate)
  (bind _returnvalue (Game|SpawnActorfromClass _firstpersonequipclass (Math|Transform|MakeTransform "0, 0, 0" "0, 0, 0" "1.000000,1.000000,1.000000") "Undefined" 0 0))
  (bind _output_get (Variables|Default|SetEquippedItemRef _returnvalue))
  (Transformation|AttachComponentToComponent _output_get (Variables|Default|GetSkeletalMesh) _socketname "SnapToTarget" "SnapToTarget" "SnapToTarget" true))

(event Custom|DequipItemEvent
  (bind _equippeditemref (Variables|Default|GetEquippedItemRef)
    (:then
      (Actor|DestroyActor _equippeditemref)
      (Variables|Default|SetEquippedState "NewEnumerator4"))
    (:else)))

(event Custom|EquipArmor
  (params (itemInfo :type S%20Item%20Info%20Structure))
  (CallFunction|EquipArmorFunction itemInfo))

(event Custom|DequipArmor
  (params (armorType :type E_ArmorType%20Enum :default "NewEnumerator0"))
  (switch Utilities|FlowControl|Switch|SwitchonE_ArmorType armorType
    (:NewEnumerator0
      (bind _chestslot (Variables|Default|GetChestSlot)
        (:then
          _)
        (:else)))
    (:NewEnumerator1
      (bind _chestslot_2 (Variables|Default|GetChestSlot)
        (:then
          _)
        (:else)))
    (:NewEnumerator2
      (bind _pantsslot (Variables|Default|GetPantsSlot)
        (:then
          _)
        (:else)))
    (:NewEnumerator3
      (bind _bootsslot (Variables|Default|GetBootsSlot)
        (:then
          _)
        (:else))))
  (Actor|DestroyActor _chestslot))

(fn ConstructionScript)

(fn EquipArmorFunction
  (params (itemInfo :type S%20Item%20Info%20Structure))
  (bind (_itemclassref _armortype) (Utilities|Struct|BreakS_ItemInfo itemInfo))
  (LocalVariables|Setarmor _armortype)
  (bind _returnvalue (Game|SpawnActorfromClass _itemclassref (Math|Transform|MakeTransform "0, 0, 0" "0, 0, 0" "1.000000,1.000000,1.000000") "Undefined" 0 0))
  (switch Utilities|FlowControl|Switch|SwitchonE_ArmorType (LocalVariables|Getarmor)
    (:NewEnumerator0
      (bind _output_get (Variables|Default|SethelmentSlot _returnvalue)))
    (:NewEnumerator1
      (bind _output_get_2 (Variables|Default|SetChestSlot _returnvalue)))
    (:NewEnumerator2
      (bind _output_get_3 (Variables|Default|SetPantsSlot _returnvalue)))
    (:NewEnumerator3
      (bind _output_get_4 (Variables|Default|SetBootsSlot _returnvalue))))
  (Transformation|AttachComponentToComponent (Utilities|Select :Index (LocalVariables|Getarmor) :NewEnumerator0 _output_get :NewEnumerator1 _output_get_2 :NewEnumerator2 _output_get_3 :NewEnumerator3 _output_get_4) (Variables|Default|GetSkeletalMesh) "None" "SnapToTarget" "SnapToTarget" "SnapToTarget" true)
  (bind _armorref (Class|BPIArmorItem|GetArmorRef(Message) (Utilities|Select :Index (LocalVariables|Getarmor) :NewEnumerator0 _output_get :NewEnumerator1 _output_get_2 :NewEnumerator2 _output_get_3 :NewEnumerator3 _output_get_4)))
  (Components|SkinnedMesh|SetLeaderPoseComponent (Variables|/Game/_Main/Blueprints/Items/BP_ArmorMaster.BP_ArmorMaster_C|GetSkeletalMesh _armorref) (Variables|Default|GetSkeletalMesh) false false))

(fn GetPlayerWindowRef
  (return self))