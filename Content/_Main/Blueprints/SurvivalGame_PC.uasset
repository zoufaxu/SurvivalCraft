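; Player controller for a survival game that owns the main HUD widget and acts as the bridge from gameplay to UI.
; BeginPlay creates W_MainWidget on both authority and remote but adds it to the viewport only on remote; Tab or I toggles the inventory, cursor and input mode.
; Events forward item slot, crafting, stat, experience, level, armor and notification updates to child widgets, with slot lookup covering only inventory and hotbar containers.
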(event Custom|UpdateStatBar
  (params (stat :type E_StatEnum%20Enum :default "NewEnumerator0") (current :type Float%20%28double-precision%29) (max :type Float%20%28double-precision%29))
  (Default|UpdateBar (Variables|/Game/_Main/Widgets/W_MainWidget.W_MainWidget_C|GetW_PlayerStatsWindow (Variables|Default|GetMainWidgetRef)) stat current max)
  (Default|UpdateStat (Variables|/Game/_Main/Widgets/InventoryWidgets/W_Inventory.W_Inventory_C|GetW_PlayerinfoWindow (Variables|/Game/_Main/Widgets/W_MainWidget.W_MainWidget_C|GetW_Inventory (Variables|Default|GetMainWidgetRef))) stat current max))

(event Custom|ResetItemSlot
  (params (container :type E_ContainerType%20Enum :default "NewEnumerator0") (index :type Integer))
  (bind _widget (CallFunction|GetInventoryWidget container index))
  (Utilities|IsValid _widget
    (:Is%20Valid
      (Default|ResetSlot _widget))))

(event Custom|ExperienceNotify
  (params (Experience :type Integer))
  (Default|AddExperienceNotification (Variables|Default|GetMainWidgetRef) Experience))

(event Custom|UpdateLevelUI
  (params (PlayerLevel :type Integer))
  (Default|UpdatePlayerLevel (Variables|/Game/_Main/Widgets/W_MainWidget.W_MainWidget_C|GetW_Inventory (Variables|Default|GetMainWidgetRef)) PlayerLevel))

(event Custom|LevelNotify
  (params (level :type Integer))
  (Default|ShowLevelUpNotification (Variables|Default|GetMainWidgetRef) level))

(event Custom|UpdateSkillPoints
  (params (SkillPoints :type Integer))
  (Default|UpdateSkillPoints (Variables|/Game/_Main/Widgets/InventoryWidgets/W_Inventory.W_Inventory_C|GetW_PlayerinfoWindow (Variables|/Game/_Main/Widgets/W_MainWidget.W_MainWidget_C|GetW_Inventory (Variables|Default|GetMainWidgetRef))) SkillPoints))

(event Custom|RemoveLevelNotify
  (Default|RemoveLevelUpNotification (Variables|Default|GetMainWidgetRef)))

(event Custom|UpdateArmorUI
  (params (armorType :type E_ArmorType%20Enum :default "NewEnumerator0") (itemInfo :type S%20Item%20Info%20Structure))
  (Default|UpdateArmorSlot (Variables|/Game/_Main/Widgets/W_MainWidget.W_MainWidget_C|GetW_Inventory (Variables|Default|GetMainWidgetRef)) armorType itemInfo))

(event Custom|RemoveArmorUI
  (params (armorType :type E_ArmorType%20Enum :default "NewEnumerator0"))
  (Default|RemoveArmorSlot (Variables|/Game/_Main/Widgets/W_MainWidget.W_MainWidget_C|GetW_Inventory (Variables|Default|GetMainWidgetRef)) armorType))

(event Custom|SetRenderMaterial
  (params (mat :type Material%20Instance%20Object%20Reference))
  (Default|SetPlayerTexture (Variables|/Game/_Main/Widgets/W_MainWidget.W_MainWidget_C|GetW_Inventory (Variables|Default|GetMainWidgetRef)) mat))

(event Custom|UpdateItemSlot
  (params (container :type E_ContainerType%20Enum :default "NewEnumerator0") (index :type Integer) (itemInfo :type S%20Item%20Info%20Structure))
  (bind _widget (CallFunction|GetInventoryWidget container index))
  (Utilities|IsValid _widget
    (:Is%20Valid
      (Default|UpdateSlot _widget itemInfo))))

(event Custom|ShowltemWidget
  (params (resourcelmage :type Texture%202D%20Object%20Reference) (ResouceQuantity :type Integer) (ResourceName :type Text))
  (Default|ShowltemCollected (Variables|Default|GetMainWidgetRef) resourcelmage ResouceQuantity ResourceName))

(event Custom|UpdateCraftStatus
  (params (CanCraft? :type Boolean))
  (Default|UpdateCraftStatus (Variables|/Game/_Main/Widgets/InventoryWidgets/W_Inventory.W_Inventory_C|GetW_CraftingWindow (Variables|/Game/_Main/Widgets/W_MainWidget.W_MainWidget_C|GetW_Inventory (Variables|Default|GetMainWidgetRef))) CanCraft?))

(event Custom|ShowCraftingProgressBar
  (Default|ShowCraftingBar (Variables|Default|GetMainWidgetRef)))

(event Custom|InventoryOnClient
  (bind _self self)
  (Default|SetInventoryVis (Variables|Default|GetMainWidgetRef) (not (Variables|Default|GetInventtoryShown?)))
  (Variables|Default|SetbShowMouseCursor (not (Variables|Default|GetInventtoryShown?)))
  (if (Variables|Default|GetInventtoryShown?)
    (Input|SetInputModeGameOnly _self false)
    (else
      (Input|SetInputModeGameandUI _self 0 "DoNotLock" true false)))
  (Variables|Default|SetInventtoryShown? (not (Variables|Default|GetInventtoryShown?))))

(event Custom|ShowOrHideDehydrated
  (params (ShowOrHide :type Boolean))
  (bind _mainwidgetref (Variables|Default|GetMainWidgetRef))
  (if ShowOrHide
    (Default|ShowDehydratedNotification _mainwidgetref)
    (else
      (Default|RemoveDehydratedNotification _mainwidgetref))))

(event Custom|ShowOrHideStarving
  (params (ShowOrHide :type Boolean))
  (bind _mainwidgetref (Variables|Default|GetMainWidgetRef))
  (if ShowOrHide
    (Default|ShowStarvingNotification _mainwidgetref)
    (else
      (Default|RemoveStarvingNotification _mainwidgetref))))

(event Custom|UpdateExperienceUI
  (params (currentExp :type Integer) (maxExp :type Integer))
  (Default|UpdateExperience (Variables|/Game/_Main/Widgets/InventoryWidgets/W_Inventory.W_Inventory_C|GetW_PlayerinfoWindow (Variables|/Game/_Main/Widgets/W_MainWidget.W_MainWidget_C|GetW_Inventory (Variables|Default|GetMainWidgetRef))) currentExp maxExp))

(event EventBeginPlay
  (Networking|SwitchHasAuthority
    (:Authority
      (Development|PrintString "Hello")
      (bind _returnvalue (UserInterface|CreateWidget "/Game/_Main/Widgets/W_MainWidget.W_MainWidget_C" self))
      (Variables|Default|SetMainWidgetRef _returnvalue))
    (:Remote
      (Development|PrintString "b")
      (bind _returnvalue_2 (UserInterface|CreateWidget "/Game/_Main/Widgets/W_MainWidget.W_MainWidget_C" self))
      (bind _output_get (Variables|Default|SetMainWidgetRef _returnvalue_2))
      (UserInterface|Viewport|AddtoViewport _output_get 0))))

(event EventTick
  (params (DeltaSeconds :type Float%20%28single-precision%29)))

(event Input|KeyboardEvents|Tab
  (params (Key :type Key%20Structure :default "None"))
  (:Pressed
    (CallFunction|InventoryonClient)))

(event Input|KeyboardEvents|I
  (params (Key :type Key%20Structure :default "None"))
  (:Pressed
    (CallFunction|InventoryonClient)))

(fn ConstructionScript)

(fn GetInventoryWidget
  (params (container :type E_ContainerType%20Enum :default "NewEnumerator0") (slotIndex :type Integer))
  (return (Utilities|Array|Get(acopy) (Variables|/Game/_Main/Widgets/InventoryWidgets/W_ItemContainerGrid.W_ItemContainerGrid_C|GetSlots (Utilities|Select :Index container :NewEnumerator0 (Variables|/Game/_Main/Widgets/InventoryWidgets/W_Inventory.W_Inventory_C|GetW_ItemContainerGrid (Variables|/Game/_Main/Widgets/W_MainWidget.W_MainWidget_C|GetW_Inventory (Variables|Default|GetMainWidgetRef))) :NewEnumerator1 (Variables|/Game/_Main/Widgets/InventoryWidgets/W_Hotbar.W_Hotbar_C|GetW_ItemContainerGrid (Variables|/Game/_Main/Widgets/W_MainWidget.W_MainWidget_C|GetW_Hotbar (Variables|Default|GetMainWidgetRef))) :NewEnumerator2 0 :NewEnumerator3 0)) slotIndex)))

(fn SurvivalGamePCRef
  (return self))