(event Custom|LaunchBuildMode
  (params (StructureID :type Integer))
  (if (Variables|Default|GetIsBuildModeEnable?)
    (CallFunction|StopBuildLoop)
    (else
      (Variables|Default|SetIsBuildModeEnable? true)
      (CallFunction|BuildModeClient (Variables|Default|GetStructureIDDebug)))))

(event Custom|BuildLoop
  (bind _buildpreview (Variables|Default|GetBuildPreview))
  (if (Variables|Default|GetIsBuildModeEnable?)
    (Utilities|FlowControl|Delay 0.01)
    (CallFunction|BuildModeClient)
    (else
      (Variables|Default|SetIsBuildModeEnable? false)
      (Utilities|IsValid _buildpreview
        (:Is%20Valid
          (Actor|DestroyActor _buildpreview))))))

(event Custom|StopBuildLoop
  (bind _buildpreview (Variables|Default|GetBuildPreview))
  (Variables|Default|SetIsBuildModeEnable? false)
  (Utilities|IsValid _buildpreview
    (:Is%20Valid
      (Actor|DestroyActor _buildpreview))))

(event Custom|SpawnBuildOnServer
  (params (transform :type Transform) (ClientCameraVector :type Vector) (ClientCameraRotation :type Rotator) (StructurelD :type Integer))
  (Networking|SwitchHasAuthority
    (:Authority
      (Variables|Default|SetBuildTransform transform)
      (bind _canbuild_ (CallFunction|BuildPlacementCheck StructurelD ClientCameraVector ClientCameraRotation))
      (if _canbuild_
        (CallFunction|SpawnBuildable transform StructurelD)
        (else
          (bind _buildpreview (Variables|Default|GetBuildPreview)
            (:then
              (Actor|DestroyActor _buildpreview))
            (:else)))))))

(fn BuildModeClient
  (params (StructureID :type Integer))
  (bind _survivalcharref (Class|BPISurvivalCharacter|GetSurvivalCharRef(Message) (Components|GetOwner)))
  (Variables|Default|GetBuildPreview
    (:then
      _)
    (:else
      (CallFunction|SpawnBuildPreview StructureID)
      (bind _buildpreview (Variables|Default|GetBuildPreview)
        (:then
          _)
        (:else))))
  (bind (_outhit _returnvalue) (Collision|LineTraceByChannel (+ (Transformation|GetWorldLocation (Variables|/Game/_Main/Blueprints/BP_FirstPersonCharacter.BP_FirstPersonCharacter_C|GetFirstPersonCamera _survivalcharref)) (* (Math|Vector|GetForwardVector (Variables|/Game/_Main/Blueprints/BP_FirstPersonCharacter.BP_FirstPersonCharacter_C|GetFirstPersonCamera _survivalcharref)) 3.5e+02)) (+ (Transformation|GetWorldLocation (Variables|/Game/_Main/Blueprints/BP_FirstPersonCharacter.BP_FirstPersonCharacter_C|GetFirstPersonCamera _survivalcharref)) (* (Math|Vector|GetForwardVector (Variables|/Game/_Main/Blueprints/BP_FirstPersonCharacter.BP_FirstPersonCharacter_C|GetFirstPersonCamera _survivalcharref)) 1e+03)) (Utilities|Struct|BreakS_Buildableinfo (Variables|/Game/_Main/Blueprints/BuildingSystem/BP_BuildableMaster.BP_BuildableMaster_C|GetBuildableinfo _buildpreview)) false (Utilities|Array|MakeArray _buildpreview) "None"))
  (if _returnvalue
    (Variables|Default|SetHit%20Actor (.HitActor (Collision|BreakHitResult _outhit)))
    (Variables|Default|SetHit%20Component (.HitComponent (Collision|BreakHitResult _outhit)))
    (bind _survivalcharref_2 (Class|BPISurvivalCharacter|GetSurvivalCharRef(Message) (Components|GetOwner)))
    (Variables|Default|SetBuildTransform (Math|Transform|MakeTransform (.ImpactPoint (Collision|BreakHitResult _outhit)) (Math|Rotator|MakeRotator 0.0 0.0 (+ (.yaw (Transformation|GetWorldRotation (Variables|/Game/_Main/Blueprints/BP_FirstPersonCharacter.BP_FirstPersonCharacter_C|GetFirstPersonCamera _survivalcharref_2))) 9e+01)) "1.000000,1.000000,1.000000"))
    (Utilities|IsValid (Variables|Default|GetBuildPreview)
      (:Is%20Valid
        (bind (_found_ _location) (CallFunction|GetSnappingPoints))
        (if _found_
          (Variables|Default|SetBuildTransform _location)
          (if (Utilities|Struct|BreakS_Buildableinfo (Variables|/Game/_Main/Blueprints/BuildingSystem/BP_BuildableMaster.BP_BuildableMaster_C|GetBuildableinfo (Variables|Default|GetBuildPreview)))
            (bind _didhit_ (CallFunction|IsBuildFloating?))
            (bind _overlapping_ (CallFunction|CheckforOverlap))
            (CallFunction|SetPreviewColor (and (not _overlapping_) _didhit_))
            (CallFunction|BuildLoop)
            (else
              (bind _overlapping__2 (CallFunction|CheckforOverlap))
              (CallFunction|SetPreviewColor (not _overlapping__2))
              (CallFunction|BuildLoop)))
          (else
            (bind _didhit__2 (CallFunction|IsBuildFloating?))
            (bind _overlapping__3 (CallFunction|CheckforOverlap))
            (CallFunction|SetPreviewColor (and (not _overlapping__3) _didhit__2))
            (CallFunction|BuildLoop))))
      (:Is%20Not%20Valid
        (CallFunction|SpawnBuildPreview)
        (CallFunction|BuildLoop)))
    (else
      (bind _survivalcharref_3 (Class|BPISurvivalCharacter|GetSurvivalCharRef(Message) (Components|GetOwner)))
      (Variables|Default|SetBuildTransform (Math|Transform|MakeTransform (.TraceEnd (Collision|BreakHitResult _outhit)) (Math|Rotator|MakeRotator 0.0 0.0 (+ (.yaw (Transformation|GetWorldRotation (Variables|/Game/_Main/Blueprints/BP_FirstPersonCharacter.BP_FirstPersonCharacter_C|GetFirstPersonCamera _survivalcharref_3))) 9e+01)) "1.000000,1.000000,1.000000"))
      (Utilities|IsValid (Variables|Default|GetBuildPreview)
        (:Is%20Valid
          (CallFunction|SetPreviewColor false)
          (CallFunction|BuildLoop))
        (:Is%20Not%20Valid
          (CallFunction|SpawnBuildPreview)
          (CallFunction|BuildLoop))))))

(fn SpawnBuildPreview
  (params (StructureID :type Integer))
  (bind _returnvalue (Utilities|GetDataTableRow "/Game/_Main/Blueprints/BuildingSystem/Misc/DT_Structures.DT_Structures" (Utilities|String|StringToName (Utilities|String|ToString(Integer) StructureID)))
    (:then
      (bind _returnvalue_2 (Game|SpawnActorfromClass (Utilities|Struct|BreakS_BuildTableInfo _returnvalue) (Variables|Default|GetBuildTransform) "Undefined" 0 0))
      (bind _output_get (Variables|Default|SetBuildPreview _returnvalue_2))
      (Collision|SetCollisionEnabled (Variables|/Game/_Main/Blueprints/BuildingSystem/BP_BuildableMaster.BP_BuildableMaster_C|GetStaticMesh _output_get) "NoCollision"))))

(fn SetPreviewColor
  (params (isGreen? :type Boolean))
  (for _array_element (Actor|GetComponentsByClass (Variables|Default|GetBuildPreview) "/Script/Engine.StaticMeshComponent")
    (for _index (range 0 (- (Rendering|Material|GetNumMaterials _array_element) 1))
      (if isGreen?
        (Rendering|Material|SetMaterial _array_element _index "/Game/_Main/Blueprints/BuildingSystem/Materials/M_Green.M_Green")
        (else
          (Rendering|Material|SetMaterial _array_element _index "/Game/_Main/Blueprints/BuildingSystem/Materials/M_Red.M_Red"))))
    (Transformation|SetWorldTransform (Variables|/Game/_Main/Blueprints/BuildingSystem/BP_BuildableMaster.BP_BuildableMaster_C|GetDefaultSceneRoot (Variables|Default|GetBuildPreview)) (Variables|Default|GetBuildTransform) false false)))

(fn SpawnBuildable
  (params (transform :type Transform) (buildIDTemp :type Integer))
  (bind _returnvalue (Utilities|GetDataTableRow "/Game/_Main/Blueprints/BuildingSystem/Misc/DT_Structures.DT_Structures" (Utilities|String|StringToName (Utilities|String|ToString(Integer) buildIDTemp)))
    (:then
      (Game|SpawnActorfromClass (Utilities|Struct|BreakS_BuildTableInfo _returnvalue) transform "Undefined" 0 0))))

(fn CheckforOverlap
  (bind _buildpreview (Variables|Default|GetBuildPreview))
  (bind _buildpreview_2 (Variables|Default|GetBuildPreview))
  (bind _buildpreview_3 (Variables|Default|GetBuildPreview))
  (bind _buildableinfo (Variables|/Game/_Main/Blueprints/BuildingSystem/BP_BuildableMaster.BP_BuildableMaster_C|GetBuildableinfo _buildpreview))
  (bind _staticmesh (Variables|/Game/_Main/Blueprints/BuildingSystem/BP_BuildableMaster.BP_BuildableMaster_C|GetStaticMesh _buildpreview_3))
  (bind _overlapboxsize (Variables|/Game/_Main/Blueprints/BuildingSystem/BP_BuildableMaster.BP_BuildableMaster_C|GetOverlapBoxSize _buildpreview_2))
  (bind (_origin _boxextent) (Collision|GetComponentBounds _staticmesh))
  (bind (_origin_2 _boxextent_2) (Collision|GetComponentBounds _overlapboxsize))
  (bind _returnvalue (select (.usecustomoverlap? _buildableinfo) _origin_2 _origin))
  (bind _returnvalue_2 (Collision|BoxTraceByChannel _returnvalue _returnvalue (/ (select (.usecustomoverlap? _buildableinfo) _boxextent_2 _boxextent) 1.2) (Math|Rotator|MakeRotator 0.0 0.0 (+ (.yaw (Transformation|GetWorldRotation (Variables|/Script/Engine.Actor|GetRootComponent (Variables|Default|GetBuildPreview)))) 9e+01)) "TraceTypeQuery1" false (Utilities|Array|MakeArray (Variables|Default|GetBuildPreview)) "None"))
  (return _returnvalue_2))

(fn BuildPlacementCheck
  (params (StructurelD :type Integer) (ClientCameraVector :type Vector) (ClientCameraRotation :type Rotator))
  (bind _survivalcharref (Class|BPISurvivalCharacter|GetSurvivalCharRef(Message) (Components|GetOwner)))
  (CallFunction|SpawnBuildPreview StructurelD)
  (bind _buildpreview (Variables|Default|GetBuildPreview)
    (:then
      (bind (_outhit _returnvalue) (Collision|LineTraceByChannel (* (Transformation|GetWorldLocation (Variables|/Game/_Main/Blueprints/BP_FirstPersonCharacter.BP_FirstPersonCharacter_C|GetFirstPersonCamera _survivalcharref)) (* ClientCameraVector 3.5e+02)) (+ (Transformation|GetWorldLocation (Variables|/Game/_Main/Blueprints/BP_FirstPersonCharacter.BP_FirstPersonCharacter_C|GetFirstPersonCamera _survivalcharref)) (* ClientCameraVector 1e+03)) (Utilities|Struct|BreakS_Buildableinfo (Variables|/Game/_Main/Blueprints/BuildingSystem/BP_BuildableMaster.BP_BuildableMaster_C|GetBuildableinfo _buildpreview)) false (Utilities|Array|MakeArray _buildpreview) "None"))
      (if _returnvalue
        (Variables|Default|SetHit%20Actor (.HitActor (Collision|BreakHitResult _outhit)))
        (Variables|Default|SetHit%20Component (.HitComponent (Collision|BreakHitResult _outhit)))
        (Variables|Default|SetBuildTransform (Math|Transform|MakeTransform (.ImpactNormal (Collision|BreakHitResult _outhit)) (Math|Rotator|MakeRotator 0.0 0.0 (+ (.yaw ClientCameraRotation) 9e+01)) "1.000000,1.000000,1.000000"))
        (Utilities|IsValid (Variables|Default|GetBuildPreview)
          (:Is%20Valid
            (bind (_found_ _location) (CallFunction|GetSnappingPoints))
            (if _found_
              (Variables|Default|SetBuildTransform _location)
              (if (Utilities|Struct|BreakS_Buildableinfo (Variables|/Game/_Main/Blueprints/BuildingSystem/BP_BuildableMaster.BP_BuildableMaster_C|GetBuildableinfo (Variables|Default|GetBuildPreview)))
                (bind _didhit_ (CallFunction|IsBuildFloating?))
                (bind _overlapping_ (CallFunction|CheckforOverlap))
                (return (and (not _overlapping_) _didhit_))
                (else
                  (bind _overlapping__2 (CallFunction|CheckforOverlap))
                  (return (not _overlapping__2))))
              (else
                (bind _didhit__2 (CallFunction|IsBuildFloating?))
                (bind _overlapping__3 (CallFunction|CheckforOverlap))
                (return (and (not _overlapping__3) _didhit__2)))))
          (:Is%20Not%20Valid
            (return false)))
        (else
          (Variables|Default|SetBuildTransform (Math|Transform|MakeTransform (.TraceEnd (Collision|BreakHitResult _outhit)) (Math|Rotator|MakeRotator 0.0 0.0 (+ (.yaw ClientCameraRotation) 9e+01)) "1.000000,1.000000,1.000000"))
          (Utilities|IsValid (Variables|Default|GetBuildPreview)
            (:Is%20Valid
              _)
            (:Is%20Not%20Valid
              _))
          (return false))))
    (:else)))

(fn GetSnappingPoints
  (bind _boxes (Class|BPIBuildinterface|ReturnBoxes(Message) (Variables|Default|GetHit%20Actor)))
  (bind _array_element (Utilities|Array|ForEachLoopwithBreak _boxes :!label _label)
    (:LoopBody
      (bind _hit_component (Variables|Default|GetHit%20Component)
        (:then
          (if (== _array_element _hit_component)
            (LocalVariables|SetlocalFound? true)
            (goto _label Break)))
        (:else)))
    (:Completed
      (bind _hit_component_2 (Variables|Default|GetHit%20Component)
        (:then
          (return (LocalVariables|GetlocalFound?) (Transformation|GetWorldTransform _hit_component_2)))
        (:else
          (return (LocalVariables|GetlocalFound?) ""))))))

(fn ChangeBuildStructure
  (bind _buildpreview (Variables|Default|GetBuildPreview)
    (:then
      (Actor|DestroyActor _buildpreview))
    (:else
      _))
  (CallFunction|SpawnBuildPreview (Variables|Default|GetStructureIDDebug)))

(fn IsBuildFloating?
  (bind _buildtransform (Variables|Default|GetBuildTransform))
  (bind _returnvalue (Collision|LineTraceByChannel (.location _buildtransform) (- (.location _buildtransform) "0.000000,0.000000,50.000000") "TraceTypeQuery1" false (Utilities|Array|MakeArray (Variables|Default|GetBuildPreview)) "None"))
  (return _returnvalue))