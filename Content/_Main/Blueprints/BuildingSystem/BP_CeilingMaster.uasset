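; BP_CeilingMaster is the base ceiling piece Blueprint in the building system.
; It overrides no gameplay events, and its construction script only runs the parent's.
; ReturnBoxes supplies an array of four Ceiling and four Wall components, apparently the boxes where neighboring ceiling and wall pieces attach.
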(event EventBeginPlay)

(event Collision|EventActorBeginOverlap
  (params (OtherActor :type Actor%20Object%20Reference)))

(event EventTick
  (params (DeltaSeconds :type Float%20%28single-precision%29)))

(fn ConstructionScript
  (|CallParentFunction))

(fn ReturnBoxes
  (return (Utilities|Array|MakeArray (Variables|Default|GetCeiling) (Variables|Default|GetCeiling1) (Variables|Default|GetCeiling2) (Variables|Default|GetCeiling3) (Variables|Default|GetWall) (Variables|Default|GetWall1) (Variables|Default|GetWall2) (Variables|Default|GetWall3))))